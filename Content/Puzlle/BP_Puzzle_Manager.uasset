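; Puzzle manager that opens a door once the count of filled slots matches the slot array's length.
; On BeginPlay it loops over Slots, with the OnSlotFilled bind call placed after the empty loop body rather than inside it.
; Each OnOneSlotFilled event increments FilledCount and, on a match, calls OpenDoor on DoorActor if that reference is valid.
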(event `self.ReceiveBeginPlay`
  (for _array_element (`|MakeArray` (`self.Slots`))
    _)
  (add `/Game/Puzlle/BP_PuzzleSlot.OnSlotFilled` _array_element (delegate `OnOneSlotFilled`)))

(event `OnOneSlotFilled`
  (bind _dooractor (`self.DoorActor`))
  (bind _result (`/Engine/EditorBlueprintResources/StandardMacros.IncrementInt` (`self.Filled Count`))
    (:`  `
      (bind _output_get (set `self.Filled Count` _result))
      (if (== (`KismetArrayLibrary.Array_Length` (`|MakeArray` (`self.Slots`))) _output_get)
        (`/Engine/EditorBlueprintResources/StandardMacros.IsValid` _dooractor
          (:`Is Valid`
            (`/Game/Puzlle/sağlıkocagi_kapi.OpenDoor` _dooractor)))))))

(fn `UserConstructionScript`)