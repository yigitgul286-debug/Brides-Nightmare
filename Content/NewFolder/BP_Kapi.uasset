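; BP_Kapi is a door that opens once enough items have been collected.
; CollectItem increments a counter, and OpenDoorCheck compares it to the required maximum, using a DoOnce so the door opens only once.
; OpeningTheDor plays the KapiAcil timeline, whose DoorRot track lerps the static mesh's yaw to swing it open.
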(event `OpeningTheDor`
  (bind (_direction _doorrot) (`Timeline|KapiAcil`)
    (:`Update`
      (`SceneComponent.K2_SetRelativeRotation` (`self.StaticMesh`) (`KismetMathLibrary.MakeRotator` 0.0 0.0 (`KismetMathLibrary.Lerp` 0.0 120.0 _doorrot)) false false))))

(event `CollectItem`
  (`/Engine/EditorBlueprintResources/StandardMacros.IncrementInt` (`self.currentItemsCollected`)))

(event `OpenDoorCheck`
  (if (>= (`self.currentItemsCollected`) (`self.MaxItemsCollected`))
    (`/Engine/EditorBlueprintResources/StandardMacros.DoOnce` false
      (:`Completed`
        (`self.OpeningTheDor`)))))

(fn `UserConstructionScript`)