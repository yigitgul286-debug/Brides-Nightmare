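; Butcher shop door Blueprint that swings open once an item count reaches its target.
; KasapKap increments Esya1, and kapiacilcak compares it to Esya2, calling kapiacils through a DoOnce when the count is met.
; kapiacils plays the KapiAcil timeline, whose DoorRot track lerps the static mesh's relative yaw to 120 degrees.
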(event `kapiacils`
  (bind (_direction _doorrot) (`Timeline|KapiAcil`)
    (:`Update`
      (`SceneComponent.K2_SetRelativeRotation` (`self.StaticMesh`) (`KismetMathLibrary.MakeRotator` 0.0 0.0 (`KismetMathLibrary.Lerp` 0.0 120.0 _doorrot)) false false))))

(event `KasapKap`
  (`/Engine/EditorBlueprintResources/StandardMacros.IncrementInt` (`self.esya1`)))

(event `kapiacilcak`
  (if (>= (`self.esya1`) (`self.esya2`))
    (`/Engine/EditorBlueprintResources/StandardMacros.DoOnce` false
      (:`Completed`
        (`self.kapiacils`)))))

(fn `UserConstructionScript`)